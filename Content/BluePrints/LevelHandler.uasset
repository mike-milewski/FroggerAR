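; LevelHandler is an AR actor that anchors the level to an assigned AR pin and shows it only while that pin is tracking.
; Each tick it teleports to the pin's position, offset along X and lowered by the frog's eye height, copying scale but not rotation.
; When tracking stops it removes and clears the pin via AssignARPin.
; SetMusic plays the looping song; game-start and HUD creation logic is unconnected.
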(event `self.ReceiveBeginPlay`)

(event `self.ReceiveTick`
  (params (DeltaSeconds :type "Float (single-precision)"))
  (bind _returnvalue (`ARPin.GetLocalToWorldTransform` (`self.ARPin`)))
  (bind _returnvalue_2 (`ARPin.GetTrackingState` (`self.ARPin`)))
  (if (`self.HasValidARPin`)
    (`|ExecutionSequence`
      (:`then_0`
        (`SceneComponent.SetVisibility` (`self.DefaultSceneRoot`) (select `EARTrackingState` _returnvalue_2 :`Tracking` true) true))
      (:`then_1`
        (switch `EARTrackingState` _returnvalue_2
          (:`Tracking`
            (`self.K2_SetActorTransform` (`KismetMathLibrary.MakeTransform` (`KismetMathLibrary.MakeVector` (+ (.x (.location _returnvalue)) 50.0) (.y (.location _returnvalue)) (- (.z (.location _returnvalue)) (`Pawn.BaseEyeHeight` (`self.FrogRef`)))) (struct) (.scale _returnvalue)) false true))
          (:`StoppedTracking`
            (`self.AssignARPin` null)))))
    (else
      (`SceneComponent.SetVisibility` (`self.DefaultSceneRoot`) false true))))

(fn `AssignARPin`
  (params (ARPin :type "ARPin Object Reference"))
  (if (`KismetSystemLibrary.IsValid` (`self.ARPin`))
    (`ARBlueprintLibrary.RemovePin` (`self.ARPin`)))
  (set `self.ARPin` ARPin))

(fn `HasValidARPin`
  (returns (HasValidARPin :type Boolean))
  (return (`KismetSystemLibrary.IsValid` (`self.ARPin`))))

(fn `SetMusic`
  (bind _audio (`self.Audio`))
  (`AudioComponent.SetSound` _audio "/Game/_Audio/Music/Song_Loop__Cue.Song_Loop__Cue")
  (`AudioComponent.Play` _audio 0.0))

(fn `UserConstructionScript`)